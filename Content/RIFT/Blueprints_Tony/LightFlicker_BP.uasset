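; Flickering light fixture actor that toggles its PointLight in irregular bursts with matching glow and audio.
; BeginPlay creates a dynamic material on the mesh, then loops on delays picked randomly from FlashTimes.
; Each toggle syncs the material's IsOn parameter to light visibility, plays a spark sound and mutes or restores the hum.
; A counter inserts a longer random pause after every eight toggles.
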(event Collision|EventActorBeginOverlap
  (params (OtherActor :type Actor%20Object%20Reference)))

(event EventBeginPlay
  (bind _hum (Variables|Default|GetHum))
  (bind _pointlight (Variables|Default|GetPointLight))
  (bind _returnvalue (Rendering|IsVisible _pointlight))
  (CallFunction|GetNewFlashTime)
  (CallFunction|CreateDynLightMat)
  (Utilities|FlowControl|Delay (Variables|Default|GetCurrentFlashTime) :!label _label)
  (Rendering|ToggleVisibility (Variables|Default|GetPointLight) false)
  (Utilities|FlowControl|Sequence
    (:then_0
      (Rendering|Material|SetScalarParameterValue (Variables|Default|GetLightMat) "IsOn" (Math|Conversions|ToFloat(Boolean) _returnvalue) :!class /Script/Engine.MaterialInstanceDynamic)
      (Audio|Components|Audio|Play (Variables|Default|GetSparkSound) 0.0)
      (if _returnvalue
        (Audio|Components|Audio|SetVolumeMultiplier _hum 1.0 :!class /Script/Engine.AudioComponent)
        (else
          (Audio|Components|Audio|SetVolumeMultiplier _hum 0.0 :!class /Script/Engine.AudioComponent))))
    (:then_1
      (CallFunction|GetNewFlashTime)
      (Math|Float|IncrementFloat (Variables|Default|GetCounter)
        (:%20%20
          (if (>= (Variables|Default|GetCounter) 8.0)
            (Utilities|FlowControl|Delay (Math|Random|RandomFloatinRange 3.0 7.0))
            (Variables|Default|SetCounter 0.0)
            (goto _label)
            (else
              (goto _label))))))))

(fn ConstructionScript)

(fn GetNewFlashTime
  (Variables|Default|SetCurrentFlashTime (Utilities|Array|Get(acopy) (Variables|Default|GetFlashTimes) (Math|Random|RandomIntegerinRange 0 (Utilities|Array|LastIndex (Variables|Default|GetFlashTimes))))))

(fn CreateDynLightMat
  (bind _returnvalue (Rendering|Material|CreateDynamicMaterialInstance (Variables|Default|GetStaticMesh) 1 0 "None" :!class /Script/Engine.PrimitiveComponent))
  (Variables|Default|SetLightMat _returnvalue))