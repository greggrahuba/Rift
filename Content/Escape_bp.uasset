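; Escape exit actor that registers itself with the DejaVu game mode and serves as the level's finish point.
; ActivateLights reveals one point light per box-hit count up to three, with the third also starting a timeline that moves the door mesh along Z.
; A second timeline rotates a spotlight from BeginPlay.
; The first overlap with EscapeDetector prints the elapsed game time and pauses the game.
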(event OnComponentBeginOverlap(EscapeDetector)
  (params (OverlappedComponent :type Primitive%20Component%20Object%20Reference) (OtherActor :type Actor%20Object%20Reference) (OtherComp :type Primitive%20Component%20Object%20Reference) (OtherBodyIndex :type Integer) (bFromSweep :type Boolean) (SweepResult :type Hit%20Result%20Structure%20%28by%20ref%29))
  (Utilities|FlowControl|DoOnce false
    (:Completed
      (Development|PrintString (Utilities|String|Append "You finished in " (Utilities|String|ToString(Float) (Utilities|Time|GetGameTimeinSeconds)) " seconds!") true true "(R=0.000000,G=0.660000,B=1.000000,A=1.000000)" 1.8e+02)
      (Game|SetGamePaused true))))

(event Custom|Activate%20Lights
  (params (Boxes%20Hit :type Integer))
  (if (== Boxes%20Hit 1)
    (Rendering|SetVisibility (Variables|Default|GetPointLight) true false)
    (elif (== Boxes%20Hit 2)
      (Rendering|SetVisibility (Variables|Default|GetPointLight1) true false)
      (elif (== Boxes%20Hit 3)
        (Rendering|SetVisibility (Variables|Default|GetPointLight2) true false)
        (bind _opening (Timeline|Open%20Door PlayFromStart)
          (:Update
            (Class|SceneComponent|AddLocalTransform (Variables|Default|GetStaticMesh) (Math|Transform|MakeTransform (Math|Vector|MakeVector 0.0 0.0 _opening) "0, 0, 0" "1,1,1") false false)))))))

(event EventBeginPlay
  (Variables|/Game/FirstPersonBP/Blueprints/DejaVu.DejaVu_C|SetEscape (.AsDeja%20Vu (Utilities|Casting|CastToDejaVu (Game|GetGameMode))) self)
  (bind _rotate (Timeline|Rotate%20Spotlight PlayFromStart)
    (:Update
      (Transformation|AddLocalRotation (Variables|Default|GetSpotLight) (Math|Rotator|MakeRotator 0.0 0.0 _rotate) false false))))

(fn ConstructionScript)